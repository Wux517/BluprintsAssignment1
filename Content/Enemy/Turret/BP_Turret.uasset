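; Enemy turret that automatically shoots at nearby pawns and explodes when its health runs out.
; Each tick it picks the closest pawn in line of sight via sphere overlap, then turns its top at constant speed with clamped pitch.
; Once cooled down and aligned by a dot-product check, a DoN loop fires two staggered left-right volleys, playing curve-driven barrel recoil timelines.
; A TakingDamage event handles health and destruction.
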(event Custom|Fire
  ;[1 1 1] Each Time the turret fires there is a total of 4 bullets being fired, 2 from each barrell, So I loop through 2 times through DO N
  (Variables|Private|SetTimeOfLastFire (Utilities|Time|GetGameTimeinSeconds))
  (Utilities|FlowControl|Sequence
    (:then_0
      (goto _label Reset))
    (:then_1
      (Utilities|FlowControl|DoN 2 :!label _label
        (:Exit
          ;[1 1 1] Comment
          (Game|SpawnActorfromClass "/Game/Enemy/Turret/BP_TurretProjectile.BP_TurretProjectile_C" (Transformation|GetSocketTransform (Variables|Default|GetStaticMeshBarrelL) "BulletSpawn" "RTS_World") "Undefined" 0 0)
          ;[1 1 1] Doing the same for the Right Barrell
          (Components|Timeline|PlayfromStart (Variables|Default|GetRecoilTimelineL))
          (Utilities|FlowControl|Delay 0.2)
          (Game|SpawnActorfromClass "/Game/Enemy/Turret/BP_TurretProjectile.BP_TurretProjectile_C" (Transformation|GetSocketTransform (Variables|Default|GetStaticMeshBarrelR) "BulletSpawn" "RTS_World") "Undefined" 0 0)
          (Components|Timeline|PlayfromStart (Variables|Default|GetRecoilTimelineR))
          (Utilities|FlowControl|Delay 0.4)
          (goto _label))))))

(event EventTakingDamage
  (params (DamageAmount :type Float%20%28double-precision%29))
  ;[1 1 1] Taking Damage Function which comunicates with the FistPersonProjectiles through Interface.
  (bind _output_get (Variables|Default|SetCurrentHealth (Math|Float|Clamp(Float) (- (Variables|Default|GetCurrentHealth) DamageAmount) 0.0 (Variables|Default|GetMaxHealth))))
  (if (not (> _output_get 0.1))
    ;[1 1 1] Spawns Explotion at Turret Death
    (Effects|SpawnEmitteratLocation "/Game/StarterContent/Particles/P_Explosion.P_Explosion" (Transformation|GetActorLocation))
    (Actor|DestroyActor)))

(event EventTick
  (params (DeltaSeconds :type Float%20%28single-precision%29))
  ;[1 1 1] Main Turret loop. Finding Target > Rotating > Shooting.
  (Private|FindBestTarget)
  (Variables|Private|GetOurTarget
    (:then
      (Private|UpdateTurretRotation DeltaSeconds)
      (Private|UpdateFire))
    (:else)))

(event EventBeginPlay
  ;[1 1 1] Setting Recoil Curves to Barrels
  (Class|TimelineComponent|SetFloatCurve (Variables|Default|GetRecoilTimelineL) "/Game/Enemy/Turret/CurveReceoil.CurveReceoil" "Recoil")
  (Class|TimelineComponent|SetFloatCurve (Variables|Default|GetRecoilTimelineR) "/Game/Enemy/Turret/CurveReceoil.CurveReceoil" "Recoil"))

(fn ConstructionScript)

(fn FindBestTarget
  ;[1 1 1] Making a SphereOverlap to use as a Targeting Range. Defining Sensing Range aswell as what it should detect.
  (LocalVariables|SetBestDistance%20%28local%29 (+ (Variables|Constants|GetSensingRange) 1.0))
  (bind _outactors (Collision|SphereOverlapActors (Transformation|GetActorLocation) (Variables|Constants|GetSensingRange) (Utilities|Array|MakeArray "ObjectTypeQuery3") "/Script/Engine.Actor"))
  ;[1 1 1] Finding Targets and looking for the closest one.
  (for _array_element _outactors
    (bind _output_get (LocalVariables|SetCurrentTarget%20%28local%29 _array_element))
    (bind _output_get_2 (LocalVariables|SetCurrentDistance%20%28local%29 (Transformation|GetDistanceTo _output_get self)))
    (if (or (< _output_get_2 (LocalVariables|GetBestDistance%20%28local%29)) (not (Utilities|IsValid (LocalVariables|GetBestTarget%20%28local%29)))) ; Closest Target So Far?
      ;[1 1 1] Looking From The turret top to the current target to see if it has line of sight, so it does not shoot if you hide, also setting the current target to the "Best target" which will be targeted.
      (bind _result (CallFunction|HasLineofSight (Transformation|GetWorldLocation (Variables|Default|GetStaticMeshTop)) (Transformation|GetActorLocation (LocalVariables|GetCurrentTarget%20%28local%29)) (Utilities|Array|MakeArray self (LocalVariables|GetCurrentTarget%20%28local%29))))
      (if _result
        (LocalVariables|SetBestTarget%20%28local%29 (LocalVariables|GetCurrentTarget%20%28local%29))
        (LocalVariables|SetBestDistance%20%28local%29 (LocalVariables|GetCurrentDistance%20%28local%29)))))
  (Variables|Private|SetOurTarget (LocalVariables|GetBestTarget%20%28local%29)))

(fn UpdateTurretRotation
  (params (DeltaSeconds :type Float%20%28double-precision%29))
  ;[1 1 1] Rotating Toward The current target, Clamped angles to avoid turret clipping through itself,
  (bind _output_get (LocalVariables|SetNewRotation (Class|KismetMathLibrary|RInterptoConstant (Transformation|GetWorldRotation (Variables|Default|GetStaticMeshTop)) (Math|Rotator|FindLookatRotation (Transformation|GetWorldLocation (Variables|Default|GetStaticMeshTop)) (Transformation|GetActorLocation (Variables|Private|GetOurTarget))) DeltaSeconds (Variables|Constants|GetRotationSpeed))))
  (Transformation|SetWorldRotation (Variables|Default|GetStaticMeshTop) (Math|Rotator|MakeRotator (Math|Float|ClampAngle (.roll _output_get) 0.0 0.0) (Math|Float|ClampAngle (.pitch _output_get) -45.0 75.0) (.yaw _output_get)) false false))

(fn UpdateFire
  ;[1 1 1] Looking at in game time to determine if the cooldown has completed.
  (if (> (- (Utilities|Time|GetGameTimeinSeconds) (Variables|Private|GetTimeOfLastFire)) (Variables|Constants|GetRateOfFire)) ; Has rate of fire cooled
    ;[1 1 1] Returning a Value between 0-1 to determine if the turret is currently aiming at the target, If it is with a small margin the turret will shoot.
    (if (> (Math|Vector|DotProduct (Math|Vector|GetUnitDirection(Vector) (Transformation|GetWorldLocation (Variables|Default|GetStaticMeshTop)) (Transformation|GetActorLocation (Variables|Private|GetOurTarget))) (Math|Vector|GetForwardVector (Variables|Default|GetStaticMeshTop))) 0.99) ; Turret facing the target
      (CallFunction|Fire))))